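; Level manager actor that randomly switches the level's reload stations on and off.
; On BeginPlay it collects every ReloadStation actor into a list and gives each a coin-flip active state.
; Tick accumulates time and re-rolls all stations whenever the ChangesIn interval elapses, updating IsActive and StateOfField.
; The initial roll resets StateOfField only for inactive stations, while later rolls set it for both outcomes.
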(event `self.ReceiveBeginPlay`
  (bind _outactors (`GameplayStatics.GetAllActorsOfClass` "/Game/Blueprints/LevelObjects/ReloadStation.ReloadStation_C"))
  (for _array_element _outactors
    (`/Engine/EditorBlueprintResources/StandardMacros.IsValid` _array_element
      (:`Is Valid`
        (`KismetArrayLibrary.Array_AddUnique` (`self.ListOfReloadStations`) _array_element))))
  (for _array_element_2 (`self.ListOfReloadStations`)
    (if (== (`KismetMathLibrary.RandomIntegerInRange` 0 1) 0)
      (set `/Game/Blueprints/LevelObjects/ReloadStation.IsActive` false _array_element_2)
      (set `/Game/Blueprints/LevelObjects/ReloadStation.StateOfField` 0.0 _array_element_2)
      (else
        (set `/Game/Blueprints/LevelObjects/ReloadStation.IsActive` true _array_element_2)))))

(event `self.ReceiveTick`
  (params (DeltaSeconds :type "Float (single-precision)"))
  (if (< (`self.WaitingTime`) (`self.ChangesIn`))
    (set `self.WaitingTime` (+ (`self.WaitingTime`) (`GameplayStatics.GetWorldDeltaSeconds`)))
    (else
      (for _array_element (`self.ListOfReloadStations`)
        (if (== (`KismetMathLibrary.RandomIntegerInRange` 0 1) 0)
          (set `/Game/Blueprints/LevelObjects/ReloadStation.IsActive` false _array_element)
          (set `/Game/Blueprints/LevelObjects/ReloadStation.StateOfField` 0.0 _array_element)
          (else
            (set `/Game/Blueprints/LevelObjects/ReloadStation.IsActive` true _array_element)
            (set `/Game/Blueprints/LevelObjects/ReloadStation.StateOfField` 1.0 _array_element))))
      (set `self.WaitingTime` 0.0))))

(fn `UserConstructionScript`)