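; Reload station that refills the player's base weapon ammo from its own energy pool while the player stands in its trigger box.
; Settings load from the STRReload struct, and ammo is written directly to the first BP_DisplayUI actor found.
; Tick drains energy during overlap, even at full ammo, and otherwise regenerates it in timed steps.
; The energy ratio drives a StateOfField material parameter on the field meshes.
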(event `self.ReceiveBeginPlay`
  (bind (_str_reload_energyatstart _str_reload_maxenergy _str_reload_reloadtime _str_reload_energyrecovered) (break `/Game/Parameters/STR_ReloadStation` (`self.STR_Reload`)))
  (set `self.Energy` _str_reload_energyatstart)
  (set `self.MaxEnergy` _str_reload_maxenergy)
  (set `self.ReloadTime` _str_reload_reloadtime)
  (set `self.EnergyRecovered` _str_reload_energyrecovered)
  (bind _outactors (`GameplayStatics.GetAllActorsOfClass` "/Game/Blueprints/WeaponsAndProjectiles/BP_DisplayUI.BP_DisplayUI_C"))
  (bind _output (`|GetArrayItem` _outactors))
  (`/Engine/EditorBlueprintResources/StandardMacros.IsValid` _output
    (:`Is Valid`
      (set `self.UI Display Ammo` _output))))

(event `self.ReceiveTick`
  (params (DeltaSeconds :type "Float (single-precision)"))
  (bind _ui_display_ammo (`self.UI Display Ammo`))
  (`|ExecutionSequence`
    (:`then_0`
      (if (`self.IsReloading`)
        (set `self.NextReloadIn` 0.0)
        (if (> (`self.Energy`) 0.0)
          (set `self.Energy` (- (`self.Energy`) (`self.EnergyRecovered`)))
          (if (< (`/Game/Blueprints/WeaponsAndProjectiles/BP_DisplayUI.CurrentBaseWeaponAmmo` _ui_display_ammo) (`/Game/Blueprints/WeaponsAndProjectiles/BP_DisplayUI.MaxBaseWeaponAmmo` _ui_display_ammo))
            (set `/Game/Blueprints/WeaponsAndProjectiles/BP_DisplayUI.CurrentBaseWeaponAmmo` (+ (`/Game/Blueprints/WeaponsAndProjectiles/BP_DisplayUI.CurrentBaseWeaponAmmo` _ui_display_ammo) (`self.EnergyRecovered`)) _ui_display_ammo)))
        (elif (>= (`self.NextReloadIn`) (`self.ReloadTime`))
          (if (< (`self.Energy`) (`self.MaxEnergy`))
            (set `self.Energy` (+ (`self.Energy`) (`self.EnergyRecovered`)))
            (set `self.NextReloadIn` 0.0))
          (else
            (set `self.NextReloadIn` (+ (`GameplayStatics.GetWorldDeltaSeconds`) (`self.NextReloadIn`)))))))
    (:`then_1`
      (set `self.StateOfField` (/ (`self.Energy`) (`self.MaxEnergy`))))
    (:`then_2`
      (if (> (`self.StateOfField`) 0.0)
        (`MeshComponent.SetScalarParameterValueOnMaterials` (`self.Cube`) "StateOfField" (`self.StateOfField`))
        (`MeshComponent.SetScalarParameterValueOnMaterials` (`self.Plane1`) "StateOfField" (`self.StateOfField`))
        (`MeshComponent.SetScalarParameterValueOnMaterials` (`self.Plane2`) "StateOfField" (`self.StateOfField`))
        (`MeshComponent.SetScalarParameterValueOnMaterials` (`self.Plane3`) "StateOfField" (`self.StateOfField`))
        (`MeshComponent.SetScalarParameterValueOnMaterials` (`self.Plane4`) "StateOfField" (`self.StateOfField`))
        (else
          (set `self.StateOfField` 0.0))))))

(event `self.Box.OnComponentBeginOverlap`
  (params (OverlappedComponent :type "PrimitiveComponent Object Reference") (OtherActor :type "Actor Object Reference") (OtherComp :type "PrimitiveComponent Object Reference") (OtherBodyIndex :type Integer) (bFromSweep :type Boolean) (SweepResult :type "HitResult Structure (by ref)"))
  (bind _asplayer (cast `/Game/Blueprints/Character/Player` OtherActor))
  (`/Engine/EditorBlueprintResources/StandardMacros.IsValid` _asplayer
    (:`Is Valid`
      (set `self.IsReloading` true))))

(event `self.Box.OnComponentEndOverlap`
  (params (OverlappedComponent :type "PrimitiveComponent Object Reference") (OtherActor :type "Actor Object Reference") (OtherComp :type "PrimitiveComponent Object Reference") (OtherBodyIndex :type Integer))
  (set `self.IsReloading` false))

(fn `UserConstructionScript`)