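; Basic melee enemy that takes its health and move speed from Stats and damages the player on Attack.
; Attack plays a montage and sound, then immediately switches the hit Box to overlap for a single player check before disabling it.
; A hit reduces player Health and sets blind and blur effects, also raising ThumbnailIntensity while health remains.
; Spawn, walk and attack sounds play as located events, with walk audio throttled by a Delay on Tick.
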(event `self.ReceiveBeginPlay`
  (bind (_stats_health _stats_movespeed) (break `/Game/Parameters/STR_BasicMob` (`self.Stats`)))
  (set `self.Health` _stats_health)
  (set `CharacterMovementComponent.MaxWalkSpeed` _stats_movespeed (`self.CharacterMovement`))
  (set `self.AttackReach` 300.0)
  (`FMODBlueprintStatics.PlayEventAtLocation` "/Game/FMOD/Events/Mob/Basic/Mob_B_Spawn.Mob_B_Spawn" (`KismetMathLibrary.Conv_VectorToTransform` (`self.K2_GetActorLocation` self))))

(event `self.ReceiveTick`
  (params (DeltaSeconds :type "Float (single-precision)"))
  (`KismetSystemLibrary.Delay` 0.15)
  (`FMODBlueprintStatics.PlayEventAtLocation` "/Game/FMOD/Events/Mob/Basic/Mob_B_Walk.Mob_B_Walk" (`KismetMathLibrary.Conv_VectorToTransform` (`self.K2_GetActorLocation` self))))

(event `self.Attack`
  (`|PlayMontage` (`self.Mesh`) "/Game/Mesh/Enemies/Basique/Basique_Attack_Montage.Basique_Attack_Montage"
    (:`then`
      (`FMODBlueprintStatics.PlayEventAtLocation` "/Game/FMOD/Events/Mob/Basic/Mob_B_Attack.Mob_B_Attack" (`KismetMathLibrary.Conv_VectorToTransform` (`self.K2_GetActorLocation` self)))
      (`PrimitiveComponent.SetCollisionProfileName` (`self.Box`) "OverlapAll" true)
      (`|ExecutionSequence`
        (:`then_0`
          (if (`PrimitiveComponent.IsOverlappingActor` (`self.Box`) (`GameplayStatics.GetPlayerPawn` 0))
            (bind _asplayer (cast `/Game/Blueprints/Character/Player` (`GameplayStatics.GetPlayerCharacter` 0)))
            (if (> (`/Game/Blueprints/Character/Player.Health` _asplayer) 0.0)
              (bind _output_get (set `/Game/Blueprints/Character/Player.Health` (- (stale _output_get) 5.0) _asplayer))
              (set `/Game/Blueprints/Character/Player.IsBlind` true _asplayer)
              (set `/Game/Blueprints/Character/Player.Blur Intensity` 7.0 _asplayer)
              (bind _output_get_2 (set `/Game/Blueprints/Character/Player.Thumbnail Intensity` (+ (stale _output_get_2) 0.125) _asplayer))
              (else
                (set `/Game/Blueprints/Character/Player.Health` 0.0 _asplayer)
                (set `/Game/Blueprints/Character/Player.IsBlind` true _asplayer)
                (set `/Game/Blueprints/Character/Player.Blur Intensity` 7.0 _asplayer)))))
        (:`then_1`
          (`PrimitiveComponent.SetCollisionProfileName` (`self.Box`) "NoCollision" true))))))

(fn `UserConstructionScript`
  (`parent.UserConstructionScript`))