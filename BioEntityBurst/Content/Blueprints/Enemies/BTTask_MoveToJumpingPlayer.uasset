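; Behavior tree task that sends an AI pawn to the ground beneath the player while the player is airborne.
; A downward Visibility line trace from the player's location supplies the hit point as the AI Move To destination.
; The task reports success as soon as the move is issued, without waiting for arrival, and fails if the player is on the ground.
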(event `self.ReceiveExecuteAI`
  (params (OwnerController :type "AIController Object Reference") (ControlledPawn :type "Pawn Object Reference"))
  (bind _returnvalue (`GameplayStatics.GetPlayerCharacter` 0))
  (bind (_returnvalue_x _returnvalue_y _returnvalue_z) (`KismetMathLibrary.BreakVector` (`Actor.K2_GetActorLocation` _returnvalue)))
  (if (not (`NavMovementComponent.IsMovingOnGround` (`Character.CharacterMovement` _returnvalue)))
    (bind _outhit (`KismetSystemLibrary.LineTraceSingle` (`KismetMathLibrary.MakeVector` _returnvalue_x _returnvalue_y _returnvalue_z) (`KismetMathLibrary.MakeVector` _returnvalue_x _returnvalue_y (- _returnvalue_z 2000.0)) "TraceTypeQuery1"))
    (`|AIMoveTo` ControlledPawn (`.Location` (`GameplayStatics.BreakHitResult` _outhit)) null 50.0
      (:`then`
        (`self.FinishExecute` true)))
    (else
      (`self.FinishExecute` false))))