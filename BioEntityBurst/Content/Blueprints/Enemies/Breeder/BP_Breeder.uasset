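; BP_Breeder is an egg-laying enemy that takes speed, health, egg count and hatch time from Stats.
; Attack plays a montage and briefly enables a hit box, damaging and blinding an overlapped player with screen blur.
; SpawnEgg plays a laying montage, decrements the egg count and spawns an Egg flagged as from a breeder.
; Audio events cover spawn and attack, with walk sounds throttled by a Delay on Tick.
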(event `self.ReceiveBeginPlay`
  (bind (_stats_health _stats_movespeed _stats_hatchtimeeggs _stats_numberofeggs) (break `/Game/Parameters/STR_Breeder` (`self.Stats`)))
  (`parent.ReceiveBeginPlay`)
  (set `CharacterMovementComponent.MaxWalkSpeed` _stats_movespeed (`self.CharacterMovement`))
  (set `self.Health` _stats_health)
  (set `self.NbEggs` _stats_numberofeggs)
  (`FMODBlueprintStatics.PlayEventAtLocation` "/Game/FMOD/Events/Mob/EggLayer/Mob_EL_Spawn.Mob_EL_Spawn" (`KismetMathLibrary.Conv_VectorToTransform` (`self.K2_GetActorLocation` self))))

(event `self.ReceiveTick`
  (params (DeltaSeconds :type "Float (single-precision)"))
  (`parent.ReceiveTick` DeltaSeconds)
  (`KismetSystemLibrary.Delay` 0.2)
  (`FMODBlueprintStatics.PlayEventAtLocation` "/Game/FMOD/Events/Mob/EggLayer/Mob_EL_Walk.Mob_EL_Walk" (`KismetMathLibrary.Conv_VectorToTransform` (`self.K2_GetActorLocation` self))))

(event `self.Attack`
  (`|PlayMontage` (`self.Mesh`) "/Game/Mesh/Enemies/Basique/Basique_Attack_Montage.Basique_Attack_Montage"
    (:`then`
      (`FMODBlueprintStatics.PlayEventAtLocation` "/Game/FMOD/Events/Mob/EggLayer/Mob_EL_Attack.Mob_EL_Attack" (`KismetMathLibrary.Conv_VectorToTransform` (`self.K2_GetActorLocation` self)))
      (`PrimitiveComponent.SetCollisionProfileName` (`self.Box`) "OverlapAll" true)
      (`|ExecutionSequence`
        (:`then_0`
          (if (`PrimitiveComponent.IsOverlappingActor` (`self.Box`) (`GameplayStatics.GetPlayerPawn` 0))
            (bind _asplayer (cast `/Game/Blueprints/Character/Player` (`GameplayStatics.GetPlayerCharacter` 0)))
            (if (> (`/Game/Blueprints/Character/Player.Health` _asplayer) 0.0)
              (bind _output_get (set `/Game/Blueprints/Character/Player.Health` (- (stale _output_get) 5.0) _asplayer))
              (set `/Game/Blueprints/Character/Player.IsBlind` true _asplayer)
              (set `/Game/Blueprints/Character/Player.Blur Intensity` 7.0 _asplayer)
              (bind _output_get_2 (set `/Game/Blueprints/Character/Player.Thumbnail Intensity` (+ (stale _output_get_2) 0.125) _asplayer))
              (else
                (set `/Game/Blueprints/Character/Player.Health` 0.0 _asplayer)
                (set `/Game/Blueprints/Character/Player.IsBlind` true _asplayer)
                (set `/Game/Blueprints/Character/Player.Blur Intensity` 7.0 _asplayer)))))
        (:`then_1`
          (`PrimitiveComponent.SetCollisionProfileName` (`self.Box`) "NoCollision" true))))))

(fn `SpawnEgg`
  (bind (_stats_health _stats_movespeed _stats_hatchtimeeggs) (break `/Game/Parameters/STR_Breeder` (`self.Stats`)))
  (`self.PlayAnimMontage` "/Game/Mesh/Enemies/Pondeur/NewImport/Pondeur_Walk_NewWeight_Anim_Pondeur_Pondeur_Ponte_Montage.Pondeur_Walk_NewWeight_Anim_Pondeur_Pondeur_Ponte_Montage")
  (set `self.NbEggs` (- (`self.NbEggs`) 1))
  (bind _returnvalue (`|SpawnActorFromClass` "/Game/Blueprints/Enemies/NestAndEggs/Egg.Egg_C" (`KismetMathLibrary.MakeTransform` (`self.K2_GetActorLocation`)) "Undefined" "OverrideRootScale" null null))
  (set `/Game/Blueprints/Enemies/NestAndEggs/Egg.FromBreeder` true _returnvalue)
  (set `/Game/Blueprints/Enemies/NestAndEggs/Egg.HatchTime` _stats_hatchtimeeggs _returnvalue))

(fn `UserConstructionScript`
  (`parent.UserConstructionScript`))