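; Behavior Tree task for enemy AI that checks whether the player is within the controlled mob's attack reach.
; It compares the MobMotherClass pawn's AttackReach to the PlayerDistance blackboard value and writes the result to the IsInReach key.
; The task result is inverted: it fails when the player is in reach and succeeds when out of reach.
; A pawn that fails the cast leaves the task without a finish call.
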(event `self.ReceiveExecuteAI`
  (params (OwnerController :type "AIController Object Reference") (ControlledPawn :type "Pawn Object Reference"))
  (bind _asmob_mother_class (cast `/Game/Blueprints/Enemies/MobMotherClass` ControlledPawn))
  (if (>= (`/Game/Blueprints/Enemies/MobMotherClass.AttackReach` _asmob_mother_class) (`BTFunctionLibrary.GetBlackboardValueAsFloat` (`self.PlayerDistance`)))
    (`BTFunctionLibrary.SetBlackboardValueAsBool` (`self.IsInReach`) true)
    (`self.FinishExecute` false)
    (else
      (`BTFunctionLibrary.SetBlackboardValueAsBool` (`self.IsInReach`))
      (`self.FinishExecute` true))))