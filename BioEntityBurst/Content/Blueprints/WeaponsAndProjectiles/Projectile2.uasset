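; Projectile actor for the player's base weapon in shotgun mode that damages basic mobs, flying mobs and nests.
; BeginPlay caches player, weapon and UI references, takes ShotgunDamage from the UI and impulses its sphere along camera forward.
; While shotgun fire is active, Tick sets its location from camera-derived direction vectors and destroys it after three seconds.
; Hits subtract Health and destroy the projectile, as do static mesh actor hits.
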(event `self.ReceiveBeginPlay`
  (bind _baseweaponreference (`self.BaseWeaponReference`))
  (bind _baseweaponreference_2 (`self.BaseWeaponReference`))
  (bind _outactors (`GameplayStatics.GetAllActorsOfClass` "/Game/Blueprints/Character/Player.Player_C"))
  (bind _output (`|GetArrayItem` _outactors))
  (`/Engine/EditorBlueprintResources/StandardMacros.IsValid` _output
    (:`Is Valid`
      (bind _output_get (set `self.PlayerReference` _output))
      (`|ExecutionSequence`
        (:`then_0`
          (bind _baseweapon (`/Game/Blueprints/Character/Player.BaseWeapon` _output_get))
          (`/Engine/EditorBlueprintResources/StandardMacros.IsValid` _baseweapon
            (:`Is Valid`
              (set `self.BaseWeaponReference` _baseweapon))))
        (:`then_1`
          (bind _outactors_2 (`GameplayStatics.GetAllActorsOfClass` "/Game/Blueprints/WeaponsAndProjectiles/BP_DisplayUI.BP_DisplayUI_C"))
          (bind _output_2 (`|GetArrayItem` _outactors_2))
          (`/Engine/EditorBlueprintResources/StandardMacros.IsValid` _output_2
            (:`Is Valid`
              (set `self.BP Display UI` _output_2))))
        (:`then_2`
          (`/Engine/EditorBlueprintResources/StandardMacros.IsValid` _baseweaponreference_2
            (:`Is Valid`
              (if (`/Game/Blueprints/WeaponsAndProjectiles/BaseWeapon2.FireWithBaseWeapon` _baseweaponreference_2)
                (if (`/Game/Blueprints/WeaponsAndProjectiles/BaseWeapon2.IsShotGun` _baseweaponreference_2)
                  (set `self.Damage` (`/Game/Blueprints/WeaponsAndProjectiles/BP_DisplayUI.ShotgunDamage` (`self.BP Display UI`))))))))
        (:`then_3`
          (`/Engine/EditorBlueprintResources/StandardMacros.IsValid` "/Game/Blueprints/WeaponsAndProjectiles/Projectile.Projectile"
            (:`Is Valid`
              (`/Engine/EditorBlueprintResources/StandardMacros.IsValid` _baseweaponreference
                (:`Is Valid`
                  (if (`/Game/Blueprints/WeaponsAndProjectiles/BaseWeapon2.FireWithBaseWeapon` _baseweaponreference)
                    (if (`/Game/Blueprints/WeaponsAndProjectiles/BaseWeapon2.IsShotGun` _baseweaponreference)
                      (`PrimitiveComponent.AddImpulse` (`self.Sphere`) (* (`KismetMathLibrary.GetForwardVector` (`PlayerCameraManager.GetCameraRotation` (`GameplayStatics.GetPlayerCameraManager` 0))) 4000.0) "None" false))))))))))))

(event `self.ReceiveTick`
  (params (DeltaSeconds :type "Float (single-precision)"))
  (bind _returnvalue (`GameplayStatics.GetPlayerCameraManager` 0))
  (bind _baseweaponreference (`self.BaseWeaponReference`))
  (`/Engine/EditorBlueprintResources/StandardMacros.IsValid` _baseweaponreference
    (:`Is Valid`
      (if (`/Game/Blueprints/WeaponsAndProjectiles/BaseWeapon2.FireWithBaseWeapon` _baseweaponreference)
        (if (`/Game/Blueprints/WeaponsAndProjectiles/BaseWeapon2.IsShotGun` _baseweaponreference)
          (`self.K2_SetActorLocation` (+ (* (`KismetMathLibrary.GetForwardVector` (`PlayerCameraManager.GetCameraRotation` _returnvalue)) (`KismetMathLibrary.Conv_DoubleToVector` 250.0)) (* (`KismetMathLibrary.Normal` (- (`SceneComponent.K2_GetComponentLocation` (`self.Sphere`)) (`PlayerCameraManager.GetCameraLocation` _returnvalue))) 240.0)))
          (bind _output_get (set `self.second` (+ (`GameplayStatics.GetWorldDeltaSeconds`) (`self.second`))))
          (if (>= _output_get 3.0)
            (`self.K2_DestroyActor`)))))))

(event `self.ReceiveHit`
  (params (MyComp :type "PrimitiveComponent Object Reference") (Other :type "Actor Object Reference") (OtherComp :type "PrimitiveComponent Object Reference") (bSelfMoved :type Boolean) (HitLocation :type "Vector Structure") (HitNormal :type "Vector Structure") (NormalImpulse :type "Vector Structure") (Hit :type "HitResult Structure (by ref)"))
  (`|ExecutionSequence`
    (:`then_0`
      (bind _asbp_basic_mobs (cast `/Game/Blueprints/Enemies/BasicMob/BP_BasicMobs` Other))
      (`/Engine/EditorBlueprintResources/StandardMacros.IsValid` _asbp_basic_mobs
        (:`Is Valid`
          (set `/Game/Blueprints/Enemies/MobMotherClass.Health` (- (`/Game/Blueprints/Enemies/MobMotherClass.Health` _asbp_basic_mobs) (`self.Damage`)) _asbp_basic_mobs)
          (`KismetSystemLibrary.PrintString` (`KismetStringLibrary.Concat_StrStr` (`KismetSystemLibrary.GetDisplayName` _asbp_basic_mobs) " has been hit by LA FRAISE !"))
          (`self.K2_DestroyActor`))))
    (:`then_1`
      (bind _asbp_flying_mob (cast `/Game/Blueprints/Enemies/FlyingMob/BP_FlyingMob` Other))
      (`/Engine/EditorBlueprintResources/StandardMacros.IsValid` _asbp_flying_mob
        (:`Is Valid`
          (set `/Game/Blueprints/Enemies/MobMotherClass.Health` (- (`/Game/Blueprints/Enemies/MobMotherClass.Health` _asbp_flying_mob) (`self.Damage`)) _asbp_flying_mob)
          (`KismetSystemLibrary.PrintString` (`KismetStringLibrary.Concat_StrStr` (`KismetSystemLibrary.GetDisplayName` _asbp_flying_mob) " has been hit by LA FRAISE !"))
          (`self.K2_DestroyActor`))))
    (:`then_2`
      (bind _asnest (cast `/Game/Blueprints/Enemies/NestAndEggs/Nest` Other))
      (`/Engine/EditorBlueprintResources/StandardMacros.IsValid` _asnest
        (:`Is Valid`
          (set `/Game/Blueprints/Enemies/MobMotherClass.Health` (- (`/Game/Blueprints/Enemies/MobMotherClass.Health` _asnest) (`self.Damage`)) _asnest)
          (`KismetSystemLibrary.PrintString` (`KismetStringLibrary.Concat_StrStr` (`KismetSystemLibrary.GetDisplayName` _asnest) " has been hit by LA FRAISE !"))
          (`self.K2_DestroyActor`))))
    (:`then_3`
      (bind _asstatic_mesh_actor (cast `StaticMeshActor` Other))
      (`/Engine/EditorBlueprintResources/StandardMacros.IsValid` _asstatic_mesh_actor
        (:`Is Valid`
          (`self.K2_DestroyActor`))))))

(fn `UserConstructionScript`)