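; BP_DisplayUI is a Blueprint that sets up the on-screen ammo and victims display when play begins.
; On BeginPlay it unpacks the STRAMMO struct into separate max, current, ratio and damage variables for rifle, shotgun and grenade.
; It then creates the UI_DisplayAmmoAndVictims widget for player 0 and adds it to the viewport.
; Tick and overlap events are unused.
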(event `self.ReceiveBeginPlay`
  (bind (_maxrifleammo _currentrifleammo _ratiorifle _rifledamage _maxshotgunammo _currentshotgunammo _ratioshotgun _shotgundamage _maxgrenadeammo _currentgrenadeammo _ratiogrenade _grenadedamage) (break `/Game/Parameters/STR_Ammo` (`self.STR AMMO`)))
  (set `self.MaxRifleAmmo` _maxrifleammo)
  (set `self.CurrentRifleAmmo` _currentrifleammo)
  (set `self.RatioRifle` _ratiorifle)
  (set `self.RifleDamage` _rifledamage)
  (set `self.MaxShotgunAmmo` _maxshotgunammo)
  (set `self.CurrentShotgunAmmo` _currentshotgunammo)
  (set `self.RatioShotgun` _ratioshotgun)
  (set `self.ShotgunDamage` _shotgundamage)
  (set `self.MaxGrenadeAmmo` _maxgrenadeammo)
  (set `self.CurrentGrenadeAmmo` _currentgrenadeammo)
  (set `self.RatioGrenade` _ratiogrenade)
  (set `self.GrenadeDamage` _grenadedamage)
  (bind _returnvalue (`|CreateWidget` "/Game/Blueprints/WeaponsAndProjectiles/UI_DisplayAmmoAndVictims.UI_DisplayAmmoAndVictims_C" (`GameplayStatics.GetPlayerController` 0)))
  (`UserWidget.AddToViewport` _returnvalue 0))

(fn `UserConstructionScript`)