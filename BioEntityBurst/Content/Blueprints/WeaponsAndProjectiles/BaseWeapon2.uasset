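; BaseWeapon2 is the player's base weapon, switching between rifle and shotgun modes and firing only while selected.
; BeginPlay caches the Player, adds the input mapping context, and finds BP_DisplayUI, which holds the ammo counts.
; Rifle shots follow the camera, rate-limited by a Tick-accumulated timer; each shotgun press sprays a loop of projectiles within a random cone.
; Firing spends UI-held ammo, reload refills the current mode, and shotgun input also clears the grenade launcher's fire flag.
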(event `self.ReceiveBeginPlay`
  (bind _grenadelauncher (`/Game/Blueprints/Character/Player.GrenadeLauncher` (`self.Player`)))
  (bind _asplayer (cast `/Game/Blueprints/Character/Player` (`self.GetOwner`)))
  (set `self.Player` _asplayer)
  (bind _asplayer_controller (cast `PlayerController` (`Pawn.GetController` _asplayer)))
  (bind _returnvalue (pcsubsystem `EnhancedInputLocalPlayerSubsystem` _asplayer_controller))
  (`/Engine/EditorBlueprintResources/StandardMacros.IsValid` _returnvalue
    (:`Is Valid`
      (`EnhancedInputSubsystemInterface.AddMappingContext` _returnvalue "/Game/Blueprints/Character/Input/IMC_Default.IMC_Default" 0 (struct))
      (bind _outactors (`GameplayStatics.GetAllActorsOfClass` "/Game/Blueprints/WeaponsAndProjectiles/BP_DisplayUI.BP_DisplayUI_C"))
      (bind _output (`|GetArrayItem` _outactors))
      (`/Engine/EditorBlueprintResources/StandardMacros.IsValid` _output
        (:`Is Valid`
          (set `self.DisplayUI` _output)
          (`/Engine/EditorBlueprintResources/StandardMacros.IsValid` _grenadelauncher
            (:`Is Valid`
              (set `self.GrenadeLauncherReference` _grenadelauncher))))))))

(event `EnhancedInput|/Game/Blueprints/Character/Input/Actions/IA_Fire`
  (params (ActionValue :type Boolean) (ElapsedSeconds :type "Float (double-precision)") (TriggeredSeconds :type "Float (double-precision)") (InputAction :type "InputAction Object Reference" :default "/Game/Blueprints/Character/Input/Actions/IA_Fire.IA_Fire"))
  (bind _displayui (`self.DisplayUI`))
  (bind _returnvalue_location (`KismetMathLibrary.BreakTransform` (`Actor.GetTransform` (`self.Player`))))
  (bind _returnvalue (`PlayerCameraManager.GetCameraRotation` (`GameplayStatics.GetPlayerCameraManager` 0)))
  (bind _currentrifleammo (`/Game/Blueprints/WeaponsAndProjectiles/BP_DisplayUI.CurrentRifleAmmo` _displayui))
  (bind _ratiorifle (`/Game/Blueprints/WeaponsAndProjectiles/BP_DisplayUI.RatioRifle` _displayui))
  (:`Triggered`
    (if (`self.IsSelected`)
      (if (`self.IsShotGun`)
        _
        (elif (> (`self.CurrentTimeInSecond`) (`self.NextRifleBulletIn`))
          (set `self.CurrentTimeInSecond` 0.0)
          (if (>= _currentrifleammo _ratiorifle)
            (set `/Game/Blueprints/WeaponsAndProjectiles/BP_DisplayUI.CurrentRifleAmmo` (- _currentrifleammo _ratiorifle) _displayui)
            (`|SpawnActorFromClass` "/Game/Blueprints/WeaponsAndProjectiles/Projectile.Projectile_C" (`KismetMathLibrary.MakeTransform` (+ _returnvalue_location (`KismetMathLibrary.GreaterGreater_VectorRotator` (`self.ProjectileOffset`) _returnvalue)) _returnvalue) "Undefined" "OverrideRootScale" null null)
            (`KismetSystemLibrary.Delay` (`self.TimeLazer`))))))))

(event `self.ReceiveTick`
  (params (DeltaSeconds :type "Float (single-precision)"))
  (set `self.CurrentTimeInSecond` (+ (`GameplayStatics.GetWorldDeltaSeconds`) (`self.CurrentTimeInSecond`))))

(event `InputAction|FireWithShotgun`
  (params (Key :type "Key Structure"))
  (bind _grenadelauncherreference (`self.GrenadeLauncherReference`))
  (bind _displayui (`self.DisplayUI`))
  (bind _currentshotgunammo (`/Game/Blueprints/WeaponsAndProjectiles/BP_DisplayUI.CurrentShotgunAmmo` _displayui))
  (bind _ratioshotgun (`/Game/Blueprints/WeaponsAndProjectiles/BP_DisplayUI.RatioShotgun` _displayui))
  (bind _returnvalue (`KismetMathLibrary.GetForwardVector` (`PlayerCameraManager.GetCameraRotation` (`GameplayStatics.GetPlayerCameraManager` 0))))
  (:`Pressed`
    (`|ExecutionSequence`
      (:`then_0`
        (set `self.FireWithBaseWeapon` true)
        (if (`self.IsSelected`)
          (if (`self.IsShotGun`)
            (if (< (`self.TimeShotGun`) 0.016667)
              (set `self.TimeShotGun` (+ (`self.TimeShotGun`) (`GameplayStatics.GetWorldDeltaSeconds`)))
              (set `self.FireWithShotgun` true)
              (if (>= _currentshotgunammo _ratioshotgun)
                (set `/Game/Blueprints/WeaponsAndProjectiles/BP_DisplayUI.CurrentShotgunAmmo` (- _currentshotgunammo _ratioshotgun) _displayui)
                (for _ (range 40)
                  (`|SpawnActorFromClass` "/Game/Blueprints/WeaponsAndProjectiles/Projectile2.Projectile2_C" (`KismetMathLibrary.MakeTransform` (+ (`Actor.K2_GetActorLocation` (`self.Player`)) (* _returnvalue 100.0)) (`KismetMathLibrary.Conv_VectorToRotator` (+ _returnvalue (`KismetMathLibrary.RandomUnitVectorInConeInDegrees` _returnvalue 55.0)))) "Undefined" "OverrideRootScale" null null)))
              (else
                (set `self.FireWithShotgun` false))))))
      (:`then_1`
        (`/Engine/EditorBlueprintResources/StandardMacros.IsValid` _grenadelauncherreference
          (:`Is Valid`
            (set `/Game/Blueprints/WeaponsAndProjectiles/GrenadeLauncher.FireWithGrenadeLauncher` false _grenadelauncherreference))))))
  (:`Released`
    (set `self.FireWithShotgun` false)
    (set `self.TimeShotGun` 0.0)))

(event `/Game/Blueprints/WeaponsAndProjectiles/Weapon.ChangeSelectedWeapon`
  (if (`self.IsSelected`)
    (set `self.IsSelected` false)
    (else
      (set `self.IsSelected` true))))

(event `EnhancedInput|/Game/Blueprints/Character/Input/Actions/IA_Reload`
  (params (ActionValue :type Boolean) (ElapsedSeconds :type "Float (double-precision)") (TriggeredSeconds :type "Float (double-precision)") (InputAction :type "InputAction Object Reference" :default "/Game/Blueprints/Character/Input/Actions/IA_Reload.IA_Reload"))
  (bind _displayui (`self.DisplayUI`))
  (bind _displayui_2 (`self.DisplayUI`))
  (:`Triggered`
    (if (`self.IsShotGun`)
      (set `/Game/Blueprints/WeaponsAndProjectiles/BP_DisplayUI.CurrentShotgunAmmo` (`/Game/Blueprints/WeaponsAndProjectiles/BP_DisplayUI.MaxShotgunAmmo` _displayui_2) _displayui_2)
      (else
        (set `/Game/Blueprints/WeaponsAndProjectiles/BP_DisplayUI.CurrentRifleAmmo` (`/Game/Blueprints/WeaponsAndProjectiles/BP_DisplayUI.MaxRifleAmmo` _displayui) _displayui)))))

(event `EnhancedInput|/Game/Blueprints/Character/Input/Actions/IA_SwitchWeapon`
  (params (ActionValue :type Boolean) (ElapsedSeconds :type "Float (double-precision)") (TriggeredSeconds :type "Float (double-precision)") (InputAction :type "InputAction Object Reference" :default "/Game/Blueprints/Character/Input/Actions/IA_SwitchWeapon.IA_SwitchWeapon"))
  (:`Triggered`
    (`/Engine/EditorBlueprintResources/StandardMacros.FlipFlop`
      (:`A`
        (set `self.IsShotGun` true))
      (:`B`
        (set `self.IsShotGun` false)))))

(fn `ChangeType`
  (if (`self.IsShotGun`)
    (set `self.IsShotGun` false)
    (else
      (set `self.IsShotGun` true))))