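; Projectile actor that flies forward and destroys itself after about three seconds.
; Each tick it sweeps along its forward vector by Speed, unscaled by delta time, and pushes Sphere and SphereCollider with impulses along the player camera's current facing.
; A timer accumulated from world delta seconds drives the destruction.
; Sphere hits only print a debug message when the other actor matches BP_BasicMobs, with no damage applied.
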(event `self.ReceiveBeginPlay`)

(event `self.ReceiveTick`
  (params (DeltaSeconds :type "Float (single-precision)"))
  (bind _returnvalue (* (`KismetMathLibrary.GetForwardVector` (`PlayerCameraManager.GetCameraRotation` (`GameplayStatics.GetPlayerCameraManager` 0))) 750.0))
  (`self.K2_SetActorLocation` self (+ (`self.K2_GetActorLocation` self) (* (`self.GetActorForwardVector` self) (`self.Speed`))) true false)
  (`PrimitiveComponent.AddImpulse` (`self.Sphere`) _returnvalue "None" false)
  (`PrimitiveComponent.AddImpulse` (`self.SphereCollider`) _returnvalue "None" false)
  (bind _output_get (set `self.second` (+ (`GameplayStatics.GetWorldDeltaSeconds`) (`self.second`))))
  (if (>= _output_get 3.0)
    (`self.K2_DestroyActor`)))

(event `self.Sphere.OnComponentHit`
  (params (HitComponent :type "PrimitiveComponent Object Reference") (OtherActor :type "Actor Object Reference") (OtherComp :type "PrimitiveComponent Object Reference") (NormalImpulse :type "Vector Structure") (Hit :type "HitResult Structure (by ref)"))
  (if (== OtherActor "/Game/Blueprints/Enemies/BasicMob/BP_BasicMobs.BP_BasicMobs")
    (`KismetSystemLibrary.PrintString` "Hello")))

(fn `UserConstructionScript`)