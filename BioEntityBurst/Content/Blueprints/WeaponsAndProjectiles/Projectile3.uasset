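; Grenade launcher projectile that deals area damage to basic mobs, flying mobs and nests.
; BeginPlay pulls damage from BP_DisplayUI and, unless homing, launches the Sphere along camera forward.
; Tick moves it forward or lerps it toward ActorToReach, keeps SphereCollider on the Sphere and enforces a lifetime.
; Hitting an enemy or static mesh briefly enables SphereCollider overlaps, which subtract Health as the blast before the actor destroys itself.
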(event `self.ReceiveBeginPlay`
  (bind _grenadelauncherreference (`self.GrenadeLauncherReference`))
  (bind _outactors (`GameplayStatics.GetAllActorsOfClass` "/Game/Blueprints/Character/Player.Player_C"))
  (bind _output (`|GetArrayItem` _outactors))
  (`/Engine/EditorBlueprintResources/StandardMacros.IsValid` _output
    (:`Is Valid`
      (bind _output_get (set `self.PlayerReference` _output))
      (`|ExecutionSequence`
        (:`then_0`
          (bind _grenadelauncher (`/Game/Blueprints/Character/Player.GrenadeLauncher` _output_get))
          (`/Engine/EditorBlueprintResources/StandardMacros.IsValid` _grenadelauncher
            (:`Is Valid`
              (set `self.GrenadeLauncherReference` _grenadelauncher))))
        (:`then_1`
          (bind _outactors_2 (`GameplayStatics.GetAllActorsOfClass` "/Game/Blueprints/WeaponsAndProjectiles/BP_DisplayUI.BP_DisplayUI_C"))
          (bind _output_2 (`|GetArrayItem` _outactors_2))
          (`/Engine/EditorBlueprintResources/StandardMacros.IsValid` _output_2
            (:`Is Valid`
              (set `self.BP Display UI` _output_2))))
        (:`then_2`
          (`/Engine/EditorBlueprintResources/StandardMacros.IsValid` _grenadelauncherreference
            (:`Is Valid`
              (if (`/Game/Blueprints/WeaponsAndProjectiles/GrenadeLauncher.FireWithGrenadeLauncher` _grenadelauncherreference)
                (set `self.Damage` (`/Game/Blueprints/WeaponsAndProjectiles/BP_DisplayUI.GrenadeDamage` (`self.BP Display UI`)))
                (if (not (`/Game/Blueprints/WeaponsAndProjectiles/GrenadeLauncher.IsHoming` (`self.GrenadeLauncherReference`)))
                  (`PrimitiveComponent.AddImpulse` (`self.Sphere`) (* (`KismetMathLibrary.GetForwardVector` (`PlayerCameraManager.GetCameraRotation` (`GameplayStatics.GetPlayerCameraManager` 0))) 50000.0) "None" false))))))))))

(event `self.ReceiveTick`
  (params (DeltaSeconds :type "Float (single-precision)"))
  (bind _returnvalue (`KismetMathLibrary.VLerp` (`self.K2_GetActorLocation`) (`self.K2_GetActorLocation` (`self.ActorToReach`)) (`self.TimeToReachTarget`)))
  (`|ExecutionSequence`
    (:`then_0`
      (if (`self.GrenadeHasExploded`)
        (bind _output_get (set `self.ExplodeIn` (+ (`self.ExplodeIn`) (`GameplayStatics.GetWorldDeltaSeconds`))))
        (if (>= _output_get 0.017)
          (`self.K2_DestroyActor`))))
    (:`then_1`
      (if (`/Game/Blueprints/WeaponsAndProjectiles/GrenadeLauncher.IsHoming` (`self.GrenadeLauncherReference`))
        (`/Engine/EditorBlueprintResources/StandardMacros.IsValid` (`self.ActorToReach`)
          (:`Is Valid`
            (set `self.TimeToReachTarget` (+ (`self.TimeToReachTarget`) (/ (`GameplayStatics.GetWorldDeltaSeconds`) 2.0)))
            (`self.K2_SetActorLocation` _returnvalue true)
            (`SceneComponent.K2_SetWorldLocation` (`self.Sphere`) _returnvalue true false)
            (if (> (`self.TimeToReachTarget`) 1.0)
              (`self.K2_DestroyActor`)))
          (:`Is Not Valid`
            (`self.K2_DestroyActor`)))
        (else
          (`/Engine/EditorBlueprintResources/StandardMacros.IsValid` (`self.Sphere`)
            (:`Is Valid`
              (`self.K2_SetActorLocation` self (+ (`self.K2_GetActorLocation` self) (* (`self.GetActorForwardVector` self) (`self.Speed`))) true false))))))
    (:`then_2`
      (`/Engine/EditorBlueprintResources/StandardMacros.IsValid` (`self.Sphere`)
        (:`Is Valid`
          (`SceneComponent.K2_SetWorldLocation` (`self.SphereCollider`) (`SceneComponent.K2_GetComponentLocation` (`self.Sphere`)) true true))))
    (:`then_3`
      (bind _output_get_2 (set `self.second` (+ (`GameplayStatics.GetWorldDeltaSeconds`) (`self.second`))))
      (if (>= _output_get_2 8.0)
        (`self.K2_DestroyActor`)))))

(event `self.ReceiveHit`
  (params (MyComp :type "PrimitiveComponent Object Reference") (Other :type "Actor Object Reference") (OtherComp :type "PrimitiveComponent Object Reference") (bSelfMoved :type Boolean) (HitLocation :type "Vector Structure") (HitNormal :type "Vector Structure") (NormalImpulse :type "Vector Structure") (Hit :type "HitResult Structure (by ref)"))
  (`/Engine/EditorBlueprintResources/StandardMacros.IsValid` "Projectile3"
    (:`Is Valid`
      (if (not (`self.GrenadeHasExploded`))
        (`|ExecutionSequence`
          (:`then_0`
            (bind _asbp_basic_mobs (cast `/Game/Blueprints/Enemies/BasicMob/BP_BasicMobs` Other))
            (`/Engine/EditorBlueprintResources/StandardMacros.IsValid` _asbp_basic_mobs
              (:`Is Valid`
                _)))
          (:`then_1`
            (bind _asbp_flying_mob (cast `/Game/Blueprints/Enemies/FlyingMob/BP_FlyingMob` Other))
            (`/Engine/EditorBlueprintResources/StandardMacros.IsValid` _asbp_flying_mob
              (:`Is Valid`
                _)))
          (:`then_2`
            (bind _asnest (cast `/Game/Blueprints/Enemies/Nest/Nest` Other))
            (`/Engine/EditorBlueprintResources/StandardMacros.IsValid` _asnest
              (:`Is Valid`
                _)))
          (:`then_3`
            (bind _asstatic_mesh_actor (cast `StaticMeshActor` Other))
            (`/Engine/EditorBlueprintResources/StandardMacros.IsValid` _asstatic_mesh_actor
              (:`Is Valid`
                _))))
        (set `self.GrenadeHasExploded` true)
        (set `PrimitiveComponent.bGenerateOverlapEvents` true (`self.SphereCollider`))))))

(event `self.SphereCollider.OnComponentBeginOverlap`
  (params (OverlappedComponent :type "PrimitiveComponent Object Reference") (OtherActor :type "Actor Object Reference") (OtherComp :type "PrimitiveComponent Object Reference") (OtherBodyIndex :type Integer) (bFromSweep :type Boolean) (SweepResult :type "HitResult Structure (by ref)"))
  (`|ExecutionSequence`
    (:`then_0`
      (bind _asbp_basic_mobs (cast `/Game/Blueprints/Enemies/BasicMob/BP_BasicMobs` OtherActor))
      (`/Engine/EditorBlueprintResources/StandardMacros.IsValid` _asbp_basic_mobs
        (:`Is Valid`
          (set `/Game/Blueprints/Enemies/MobMotherClass.Health` (- (`/Game/Blueprints/Enemies/MobMotherClass.Health` _asbp_basic_mobs) (`self.Damage`)) _asbp_basic_mobs)
          (`KismetSystemLibrary.PrintString` (`KismetStringLibrary.Concat_StrStr` (`KismetSystemLibrary.GetDisplayName` _asbp_basic_mobs) " has been hit by LA FRAISE !")))))
    (:`then_1`
      (bind _asbp_flying_mob (cast `/Game/Blueprints/Enemies/FlyingMob/BP_FlyingMob` OtherActor))
      (`/Engine/EditorBlueprintResources/StandardMacros.IsValid` _asbp_flying_mob
        (:`Is Valid`
          (set `/Game/Blueprints/Enemies/MobMotherClass.Health` (- (`/Game/Blueprints/Enemies/MobMotherClass.Health` _asbp_flying_mob) (`self.Damage`)) _asbp_flying_mob)
          (`KismetSystemLibrary.PrintString` (`KismetStringLibrary.Concat_StrStr` (`KismetSystemLibrary.GetDisplayName` _asbp_flying_mob) " has been hit by LA FRAISE !")))))
    (:`then_2`
      (bind _asnest (cast `/Game/Blueprints/Enemies/Nest/Nest` OtherActor))
      (`/Engine/EditorBlueprintResources/StandardMacros.IsValid` _asnest
        (:`Is Valid`
          (set `/Game/Blueprints/Enemies/MobMotherClass.Health` (- (`/Game/Blueprints/Enemies/MobMotherClass.Health` _asnest) (`self.Damage`)) _asnest)
          (`KismetSystemLibrary.PrintString` (`KismetStringLibrary.Concat_StrStr` (`KismetSystemLibrary.GetDisplayName` _asnest) " has been hit by LA FRAISE !")))))))

(fn `UserConstructionScript`)