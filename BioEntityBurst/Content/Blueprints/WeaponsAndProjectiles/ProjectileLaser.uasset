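; A laser projectile actor that damages mobs on contact.
; Each tick it sweeps forward a fixed step along its forward vector, independent of frame time, and destroys itself once its lifetime timer reaches MaxTime.
; On overlap it applies damage to MobMotherClass actors, prints a debug hit message and destroys itself.
; Other overlaps also destroy it, except other lasers, the Player class and ReloadStation.
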(event `self.ReceiveTick`
  (params (DeltaSeconds :type "Float (single-precision)"))
  (`self.K2_SetActorLocation` self (+ (`self.K2_GetActorLocation` self) (* (`self.GetActorForwardVector` self) 150.0)) true false)
  (bind _output_get (set `self.Timer` (+ DeltaSeconds (`self.Timer`))))
  (if (>= _output_get (`self.MaxTime`))
    (`self.K2_DestroyActor`)))

(event `self.ReceiveActorBeginOverlap`
  (params (OtherActor :type "Actor Object Reference"))
  (bind _returnvalue (`GameplayStatics.GetObjectClass` OtherActor))
  (bind _asmob_mother_class (cast `/Game/Blueprints/Enemies/MobMotherClass` OtherActor)
    (:`then`
      (`/Game/Blueprints/Enemies/MobMotherClass.TakeDamage` _asmob_mother_class (`self.Damage`))
      (`KismetSystemLibrary.PrintString` (`KismetStringLibrary.Concat_StrStr` (`KismetSystemLibrary.GetDisplayName` OtherActor) " has been hit by LA FRAISE !"))
      (`self.K2_DestroyActor`))
    (:`CastFailed`
      (cast `/Game/Blueprints/WeaponsAndProjectiles/ProjectileLaser` OtherActor
        (:`CastFailed`
          (if (and (!= _returnvalue "/Game/Blueprints/Character/Player.Player_C") (!= _returnvalue "/Game/Blueprints/LevelObjects/ReloadStation.ReloadStation_C"))
            (`self.K2_DestroyActor`)))))))

(fn `UserConstructionScript`)