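; BaseWeapon is a base weapon Blueprint, owned by the Player, that fires projectiles from Enhanced Input.
; BeginPlay caches the Player and adds the default mapping context to its controller.
; While selected and not in shotgun mode, IA_Fire spawns a projectile at a camera-rotated offset from the player, aimed along the camera; the trailing Delay gates nothing.
; Selection and shotgun mode are toggled booleans, with no shotgun firing implemented here.
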(event `self.ReceiveBeginPlay`
  (bind _asplayer (cast `/Game/Blueprints/Character/Player` (`self.GetOwner`)))
  (set `self.Player` _asplayer)
  (bind _asplayer_controller (cast `PlayerController` (`Pawn.GetController` _asplayer)))
  (bind _returnvalue (pcsubsystem `EnhancedInputLocalPlayerSubsystem` _asplayer_controller))
  (`/Engine/EditorBlueprintResources/StandardMacros.IsValid` _returnvalue
    (:`Is Valid`
      (`EnhancedInputSubsystemInterface.AddMappingContext` _returnvalue "/Game/Blueprints/Character/Input/IMC_Default.IMC_Default" 0 (struct)))))

(event `EnhancedInput|/Game/Blueprints/Character/Input/Actions/IA_Fire`
  (params (ActionValue :type Boolean) (ElapsedSeconds :type "Float (double-precision)") (TriggeredSeconds :type "Float (double-precision)") (InputAction :type "InputAction Object Reference" :default "/Game/Blueprints/Character/Input/Actions/IA_Fire.IA_Fire"))
  (bind _returnvalue_location (`KismetMathLibrary.BreakTransform` (`Actor.GetTransform` (`self.Player`))))
  (bind _returnvalue (`PlayerCameraManager.GetCameraRotation` (`GameplayStatics.GetPlayerCameraManager` 0)))
  (:`Triggered`
    (if (`self.IsSelected`)
      (if (not (`self.IsShotGun`))
        (`|SpawnActorFromClass` "/Game/Blueprints/WeaponsAndProjectiles/Projectile.Projectile_C" (`KismetMathLibrary.MakeTransform` (+ _returnvalue_location (`KismetMathLibrary.GreaterGreater_VectorRotator` (`self.ProjectileOffset`) _returnvalue)) _returnvalue) "Undefined" "OverrideRootScale" null null)
        (`KismetSystemLibrary.Delay` (`self.TimeLazer`))))))

(event `/Game/Blueprints/WeaponsAndProjectiles/Weapon.ChangeSelectedWeapon`
  (if (`self.IsSelected`)
    (set `self.IsSelected` false)
    (else
      (set `self.IsSelected` true))))

(fn `ChangeType`
  (if (`self.IsShotGun`)
    (set `self.IsShotGun` false)
    (else
      (set `self.IsShotGun` true))))