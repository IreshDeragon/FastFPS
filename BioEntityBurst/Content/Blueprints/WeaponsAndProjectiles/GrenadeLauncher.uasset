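; Grenade launcher Blueprint that fires homing Projectile3 missiles at on-screen enemies.
; BeginPlay caches the player, display UI and launcher struct settings; a separate input toggles homing.
; With homing on, firing spends UI-held ammo and spawns a camera-aimed missile for each recently rendered MobMotherClass actor, excluding NestManager.
; Tick runs the reload timer, but only disconnected target-list and single-shot branches clear GrenadeReady.
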(event `self.ReceiveBeginPlay`
  (bind (_str_grenadelauncher_timelazer _str_grenadelauncher_projectileoffset _str_grenadelauncher_nextmissilein) (break `/Game/Parameters/STR_GrenadeLauncher` (`self.STR_GrenadeLauncher`)))
  (bind _outactors (`GameplayStatics.GetAllActorsOfClass` "/Game/Blueprints/WeaponsAndProjectiles/BP_DisplayUI.BP_DisplayUI_C"))
  (bind _output (`|GetArrayItem` _outactors))
  (`/Engine/EditorBlueprintResources/StandardMacros.IsValid` _output
    (:`Is Valid`
      (set `self.BP Display UI` _output)
      (bind _outactors_2 (`GameplayStatics.GetAllActorsOfClass` "/Game/Blueprints/Character/Player.Player_C"))
      (bind _output_2 (`|GetArrayItem` _outactors_2))
      (`/Engine/EditorBlueprintResources/StandardMacros.IsValid` _output_2
        (:`Is Valid`
          (bind _output_get (set `self.Player` _output_2))
          (bind _baseweapon (`/Game/Blueprints/Character/Player.BaseWeapon` _output_get))
          (`/Engine/EditorBlueprintResources/StandardMacros.IsValid` _baseweapon
            (:`Is Valid`
              (set `self.Base Weapon Reference` _baseweapon)
              (set `self.TimeLazer` _str_grenadelauncher_timelazer)
              (set `self.ProjectileOffset` _str_grenadelauncher_projectileoffset)
              (set `self.NextMissileIn` _str_grenadelauncher_nextmissilein))))))))

(event `InputAction|FireWithGrenadeLauncher`
  (params (Key :type "Key Structure"))
  (bind _bp_display_ui (`self.BP Display UI`))
  (bind _returnvalue_location (`KismetMathLibrary.BreakTransform` (`Actor.GetTransform` (`self.Player`))))
  (bind _ratiogrenade (`/Game/Blueprints/WeaponsAndProjectiles/BP_DisplayUI.RatioGrenade` _bp_display_ui))
  (:`Pressed`
    (if (`self.GrenadeReady`)
      (set `self.FireWithGrenadeLauncher` true)
      (if (and (>= (`/Game/Blueprints/WeaponsAndProjectiles/BP_DisplayUI.CurrentGrenadeAmmo` _bp_display_ui) _ratiogrenade) (`self.IsHoming`))
        (set `/Game/Blueprints/WeaponsAndProjectiles/BP_DisplayUI.CurrentGrenadeAmmo` (- (`/Game/Blueprints/WeaponsAndProjectiles/BP_DisplayUI.CurrentGrenadeAmmo` _bp_display_ui) _ratiogrenade) _bp_display_ui)
        (bind _outactors (`GameplayStatics.GetAllActorsOfClass` "/Game/Blueprints/Enemies/MobMotherClass.MobMotherClass_C"))
        (for _array_element _outactors
          (if (!= (`GameplayStatics.GetObjectClass` _array_element) "/Game/Blueprints/Enemies/Nest/NestManager.NestManager_C")
            (`KismetSystemLibrary.PrintString` "nearly good")
            (if (`Actor.WasRecentlyRendered` _array_element 0.1)
              (`KismetSystemLibrary.PrintString` (`KismetSystemLibrary.GetObjectName` _array_element))
              (bind _returnvalue (`|SpawnActorFromClass` "/Game/Blueprints/WeaponsAndProjectiles/Projectile3.Projectile3_C" (`KismetMathLibrary.MakeTransform` (+ _returnvalue_location (`KismetMathLibrary.GreaterGreater_VectorRotator` (`self.ProjectileOffset`) (`PlayerCameraManager.GetCameraRotation` (`GameplayStatics.GetPlayerCameraManager` 0)))) (`PlayerCameraManager.GetCameraRotation` (`GameplayStatics.GetPlayerCameraManager` 0))) "Undefined" "OverrideRootScale" null null))
              (set `/Game/Blueprints/WeaponsAndProjectiles/Projectile3.ActorToReach` _array_element _returnvalue)
              (`KismetSystemLibrary.Delay` (`self.TimeLazer`))))))))
  (:`Released`
    (set `self.FireWithGrenadeLauncher` false)))

(event `InputAction|HomingMissiles`
  (params (Key :type "Key Structure"))
  (:`Pressed`
    (`/Engine/EditorBlueprintResources/StandardMacros.FlipFlop`
      (:`A`
        (set `self.IsHoming` true))
      (:`B`
        (set `self.IsHoming` false)))))

(event `self.ReceiveTick`
  (params (DeltaSeconds :type "Float (single-precision)"))
  (if (not (`self.GrenadeReady`))
    (set `self.TimeGrenadeLauncher` (+ (`GameplayStatics.GetWorldDeltaSeconds`) (`self.TimeGrenadeLauncher`)))
    (if (>= (`self.TimeGrenadeLauncher`) (`self.NextMissileIn`))
      (set `self.GrenadeReady` true)
      (set `self.TimeGrenadeLauncher` 0.0))
    (else
      (set `self.TimeGrenadeLauncher` 0.0))))